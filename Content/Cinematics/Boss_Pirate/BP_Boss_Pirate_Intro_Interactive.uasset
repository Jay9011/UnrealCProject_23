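; Interactable trigger for the Pirate boss intro that offers an "열기" (Open) prompt to the player.
; Box overlap registers the actor as target on the player's CInteractiveComponent if the player is idle, and clears it on exit.
; Interaction queries return itself as target and allow use only while the player's state component reports idle.
; No interaction response or cinematic playback is implemented in this graph.
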(event `self.Box.OnComponentBeginOverlap`
  (params (OverlappedComponent :type "PrimitiveComponent Object Reference") (OtherActor :type "Actor Object Reference") (OtherComp :type "PrimitiveComponent Object Reference") (OtherBodyIndex :type Integer) (bFromSweep :type Boolean) (SweepResult :type "HitResult Structure (by ref)"))
  (bind _ascplayer (cast `CPlayer` OtherActor))
  (bind _returnvalue (`self.GetComponentByClass` _ascplayer "/Script/CProject.CInteractiveComponent"))
  (`/Engine/EditorBlueprintResources/StandardMacros.IsValid` _returnvalue
    (:`Is Valid`
      (if (`CStateComponent.IsIdleMode` (`CBaseCharacter.State` _ascplayer))
        (`CInteractiveComponent.SetTarget` _returnvalue self self)))))

(event `self.Box.OnComponentEndOverlap`
  (params (OverlappedComponent :type "PrimitiveComponent Object Reference") (OtherActor :type "Actor Object Reference") (OtherComp :type "PrimitiveComponent Object Reference") (OtherBodyIndex :type Integer))
  (bind _ascplayer (cast `CPlayer` OtherActor))
  (bind _returnvalue (`self.GetComponentByClass` _ascplayer "/Script/CProject.CInteractiveComponent"))
  (`/Engine/EditorBlueprintResources/StandardMacros.IsValid` _returnvalue
    (:`Is Valid`
      (`CInteractiveComponent.ClearTarget` _returnvalue self))))

(fn `CanInteract`
  (params (InInteractPlayer :type "CPlayer Object Reference"))
  (returns (ReturnValue :type Boolean))
  (bind _returnvalue (`self.GetComponentByClass` InInteractPlayer "/Script/CProject.CStateComponent"))
  (`/Engine/EditorBlueprintResources/StandardMacros.IsValid` _returnvalue
    (:`Is Valid`
      (return (`CStateComponent.IsIdleMode` _returnvalue)))))

(fn `GetInteractTarget`
  (returns (ReturnValue :type "Actor Object Reference"))
  (return self))

(fn `GetInteractText`
  (returns (ReturnValue :type Text))
  (return "열기"))

(fn `UserConstructionScript`)