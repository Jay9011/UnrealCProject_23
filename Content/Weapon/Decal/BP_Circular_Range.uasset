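; BP_Circular_Range is a circular range indicator that fills over time, then plays a smash effect and removes itself.
; On BeginPlay it creates dynamic material instances for the Circle and Area components and initializes their range parameters.
; After a short delay, the Fill_Circle timeline drives the Area material's range parameter.
; When the timeline finishes, it briefly waits, spawns the P_Smash emitter at its location and destroys the actor.
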(event `self.ReceiveBeginPlay`
  (`|ExecutionSequence`
    (:`then_0`
      (bind _returnvalue (`DecalComponent.CreateDynamicMaterialInstance` (`self.Circle`)))
      (bind _output_get (set `self.CircleRef` _returnvalue))
      (`MaterialInstanceDynamic.SetScalarParameterValue` _output_get (`self.CircleRangeParamName`) 1.0))
    (:`then_1`
      (bind _returnvalue_2 (`DecalComponent.CreateDynamicMaterialInstance` (`self.Area`)))
      (bind _output_get_2 (set `self.AreaRef` _returnvalue_2))
      (`MaterialInstanceDynamic.SetScalarParameterValue` _output_get_2 (`self.CircleRangeParamName`) 0.0))
    (:`then_2`
      (`KismetSystemLibrary.Delay` 0.2)
      (bind (_direction _areavalue) (`Timeline|Fill_Circle` :!via `PlayFromStart`)
        (:`Update`
          (`MaterialInstanceDynamic.SetScalarParameterValue` (`self.AreaRef`) (`self.AreaRangeParamName`) _areavalue))
        (:`Finished`
          (`KismetSystemLibrary.Delay` 0.1)
          (`GameplayStatics.SpawnEmitterAtLocation` "/Game/HDParticlePack/Particles/P_Smash.P_Smash" (`self.K2_GetActorLocation`))
          (`self.K2_DestroyActor`))))))

(fn `UserConstructionScript`)