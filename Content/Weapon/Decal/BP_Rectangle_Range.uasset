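; BP_Rectangle_Range is a self-destroying area indicator, apparently a rectangular decal, that fills up before a smash effect plays.
; On BeginPlay it creates a dynamic material instance on its Area component, then starts the Fill_Circle timeline after a short delay.
; The timeline drives the material's range parameter; when it finishes, the actor briefly waits, spawns the P_Smash emitter at its location and destroys itself.
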(event `self.ReceiveBeginPlay`
  (`|ExecutionSequence`
    (:`then_0`
      (bind _returnvalue (`DecalComponent.CreateDynamicMaterialInstance` (`self.Area`)))
      (set `self.AreaRef` _returnvalue))
    (:`then_1`
      (`KismetSystemLibrary.Delay` 0.2)
      (bind (_direction _areavalue) (`Timeline|Fill_Circle` :!via `PlayFromStart`)
        (:`Update`
          (`MaterialInstanceDynamic.SetScalarParameterValue` (`self.AreaRef`) (`self.AreaRangeParamName`) _areavalue))
        (:`Finished`
          (`KismetSystemLibrary.Delay` 0.1)
          (`GameplayStatics.SpawnEmitterAtLocation` "/Game/HDParticlePack/Particles/P_Smash.P_Smash" (`self.K2_GetActorLocation`))
          (`self.K2_DestroyActor`))))))

(fn `UserConstructionScript`)