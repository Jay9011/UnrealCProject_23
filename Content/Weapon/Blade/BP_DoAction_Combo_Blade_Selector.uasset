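; Blade weapon combo selector action that routes the attack input to a ground or air combo.
; On BeginPlay it creates Ground and Air blade combo actions via AddDoActionCombo, passing ComboState only to the ground one, which is created only if that state is valid.
; DoAction checks whether the owner's movement is falling and forwards to the matching child action if it exists.
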(event `self.BP_BeginPlay`
  (`|ExecutionSequence`
    (:`then_0`
      (bind _combostate (`self.ComboState`)
        (:`then`
          (bind _returnvalue (`self.BP_AddDoAction_Combo` "/Game/Weapon/Blade/DoAction/BP_DoAction_Combo_Blade_Ground.BP_DoAction_Combo_Blade_Ground_C" _combostate))
          (bind _asbp_do_action_combo_blade_ground (cast `/Game/Weapon/Blade/DoAction/BP_DoAction_Combo_Blade_Ground` _returnvalue))
          (set `self.DoAction_Ground` _asbp_do_action_combo_blade_ground))
        (:`else`)))
    (:`then_1`
      (bind _returnvalue_2 (`self.BP_AddDoAction_Combo` "/Game/Weapon/Blade/DoAction/BP_DoAction_Combo_Blade_Air.BP_DoAction_Combo_Blade_Air_C"))
      (bind _asbp_do_action_combo_blade_air (cast `/Game/Weapon/Blade/DoAction/BP_DoAction_Combo_Blade_Air` _returnvalue_2))
      (set `self.DoAction_Air` _asbp_do_action_combo_blade_air))))

(event `self.DoAction`
  (if (`NavMovementComponent.IsFalling` (`Character.CharacterMovement` (`self.GetOwnerCharacter`)))
    (bind _doaction_air (`self.DoAction_Air`)
      (:`then`
        (`self.DoAction` _doaction_air))
      (:`else`))
    (else
      (bind _doaction_ground (`self.DoAction_Ground`)
        (:`then`
          (`self.DoAction` _doaction_ground))
        (:`else`)))))